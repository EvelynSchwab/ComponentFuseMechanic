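; Player character for the Fuse mechanic, mapping Enhanced Input to a FuseComponent that searches, grabs, moves, rotates, fuses and detaches objects, with jumping blocked while fusing.
; Fuse state changes switch camera and rotation behavior and toggle Niagara searching decals.
; A looping timer eases the camera socket offset and MPC_Fuse IsFusing value, while Tick fits spring arm length to the held object.
; Also spawns the Fuse HUD and provides debug readouts and an activation test key.
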(event `Key|R`
  (params (Key :type "Key Structure"))
  ;[0 0.154 0.046] Test function for activatable objects
  (:`Pressed`
    (bind _outactors (`GameplayStatics.GetAllActorsOfClass` "/Game/Fuse/Props/BP_TestActivatable.BP_TestActivatable_C"))
    (for _array_element _outactors
      (`/Game/Fuse/Props/BP_TestActivatable.Activate` _array_element))))

(event `self.ReceiveBeginPlay`
  ;[0 0.154 0.046] Set timer to update interp values InterpValueUpdateSteps/second
  (`KismetSystemLibrary.K2_SetTimer` null "UpdateInterpValues" (`self.GetValueInterpTargetDeltaSeconds`) true)
  ;[0 0.154 0.046] Cache some initial values
  (`self.SetDefaultValues`)
  ;[0 0.154 0.046] Spawn fuse HUD
  (bind _returnvalue (`|CreateWidget` "/Game/Fuse/WBP_Fuse_HUD.WBP_Fuse_HUD_C" (`GameplayStatics.GetPlayerController` 0)))
  (`UserWidget.AddToViewport` _returnvalue 0))

(event `self.ReceiveTick`
  (params (DeltaSeconds :type "Float (single-precision)"))
  (`|ExecutionSequence`
    (:`then_0`
      ;[0 0.154 0.046] Adjust the values on the spring arm
      (`self.AdjustSpringArm` DeltaSeconds))
    (:`then_1`
      ;[0 0.154 0.046] Draw additional fuse debug info, if f.drawdebugfuser is 1
      (`self.IsFuseComponentInDebug`
        (:`true`
          (`self.DrawDebugInfo` DeltaSeconds))))))

(event `EnhancedInput|/Game/ThirdPerson/Input/Actions/IA_Jump`
  (params (ActionValue :type Boolean) (ElapsedSeconds :type "Float (double-precision)") (TriggeredSeconds :type "Float (double-precision)") (InputAction :type "InputAction Object Reference" :default "/Game/ThirdPerson/Input/Actions/IA_Jump.IA_Jump"))
  ;[0 0.154 0.046] Block jump if fusing
  (:`Started`
    (`self.IsCurrentlyFusing`
      (:`NotFusing`
        (`self.Jump`)))))

(event `self.FuseComponent.OnFuserStateChanged`
  (params (NewState :type "EFuserState Enum" :default "FSTATE_NONE") (PreviousState :type "EFuserState Enum" :default "FSTATE_NONE"))
  ;[0 0.154 0.046] OnFuseStateChanged, update fuse effects
  (`self.UpdateFuseVisuals` NewState PreviousState))

(event `EnhancedInput|/Game/Fuse/Input/IA_Fuse_Toggle`
  (params (ActionValue :type Boolean) (ElapsedSeconds :type "Float (double-precision)") (TriggeredSeconds :type "Float (double-precision)") (InputAction :type "InputAction Object Reference" :default "/Game/Fuse/Input/IA_Fuse_Toggle.IA_Fuse_Toggle"))
  ;[0 0.154 0.046] Toggle fuse searching mode
  (:`Started`
    (`self.SwitchOnFusingState`
      (:`Not Fusing`
        (`FFuseComponent.TryStartSearching` (`self.FuseComponent`)))
      (:`Searching`
        (`FFuseComponent.TryStopSearching` (`self.FuseComponent`) :!label _label))
      (:`Fusing`
        (goto _label)))))

(event `EnhancedInput|/Game/Fuse/Input/IA_Fuse_Pickup`
  (params (ActionValue :type Boolean) (ElapsedSeconds :type "Float (double-precision)") (TriggeredSeconds :type "Float (double-precision)") (InputAction :type "InputAction Object Reference" :default "/Game/Fuse/Input/IA_Fuse_Pickup.IA_Fuse_Pickup"))
  ;[0 0.154 0.046] Try and pick up a targeted fuse object
  (:`Started`
    (`self.SwitchOnFusingState`
      (:`Searching`
        (`FFuseComponent.TryGrabTargetedFusable` (`self.FuseComponent`)))
      (:`Fusing`
        (`FFuseComponent.TryFuseObjects` (`self.FuseComponent`))))))

(event `EnhancedInput|/Game/Fuse/Input/IA_Fuse_Distance`
  (params (ActionValue :type "Float (double-precision)") (ElapsedSeconds :type "Float (double-precision)") (TriggeredSeconds :type "Float (double-precision)") (InputAction :type "InputAction Object Reference" :default "/Game/Fuse/Input/IA_Fuse_Distance.IA_Fuse_Distance"))
  ;[0 0.154 0.046] Adjust the fuse target distance
  (:`Started`
    (`FFuseComponent.AdjustGrabbedComponentTargetDistance` (`self.FuseComponent`) ActionValue)))

(event `EnhancedInput|/Game/Fuse/Input/IA_Fuse_Rotate`
  (params (ActionValue :type "Vector2D Structure") (ElapsedSeconds :type "Float (double-precision)") (TriggeredSeconds :type "Float (double-precision)") (InputAction :type "InputAction Object Reference" :default "/Game/Fuse/Input/IA_Fuse_Rotate.IA_Fuse_Rotate"))
  ;[0 0.154 0.046] Update held component rotation
  (:`Started`
    (`FFuseComponent.AdjustGrabbedComponentTargetRotation` (`self.FuseComponent`) ActionValue_Y ActionValue_X)))

(event `EnhancedInput|/Game/Fuse/Input/IA_Fuse_Height`
  (params (ActionValue :type "Float (double-precision)") (ElapsedSeconds :type "Float (double-precision)") (TriggeredSeconds :type "Float (double-precision)") (InputAction :type "InputAction Object Reference" :default "/Game/Fuse/Input/IA_Fuse_Height.IA_Fuse_Height"))
  ;[0 0.154 0.046] Adjust the fuse target height
  (:`Triggered`
    (`self.SwitchOnFusingState`
      (:`Fusing`
        (`FFuseComponent.AdjustGrabbedComponentTargetHeight` (`self.FuseComponent`) ActionValue)))))

(event `EnhancedInput|/Game/Fuse/Input/IA_Fuse_Detach`
  (params (ActionValue :type Boolean) (ElapsedSeconds :type "Float (double-precision)") (TriggeredSeconds :type "Float (double-precision)") (InputAction :type "InputAction Object Reference" :default "/Game/Fuse/Input/IA_Fuse_Detach.IA_Fuse_Detach"))
  ;[0 0.154 0.046] Detach the grabbed component from other actors
  (:`Started`
    (`FFuseComponent.TryDetachGrabbedComponent` (`self.FuseComponent`))))

(fn `AdjustSpringArm`
  (params (DeltaTime :type "Float (double-precision)"))
  (`|ExecutionSequence`
    (:`then_0`
      (`/Engine/EditorBlueprintResources/StandardMacros.IsValid` (`PhysicsHandleComponent.GetGrabbedComponent` (`self.FuseComponent`))
        (:`Is Valid`
          ;[0 0.154 0.046] Calculate and interp the spring arm distance
          (set `SpringArmComponent.TargetArmLength` (`KismetMathLibrary.FInterpTo` (`SpringArmComponent.TargetArmLength` (`self.CameraBoom`)) (`KismetMathLibrary.SelectFloat` (+ (+ (* (`KismetMathLibrary.Vector_Distance` (* (`self.K2_GetActorLocation`) (0.0 0.0 1.0)) (* (`SceneComponent.K2_GetComponentLocation` (`PhysicsHandleComponent.GetGrabbedComponent` (`self.FuseComponent`))) (0.0 0.0 1.0))) 1.5) (/ (`KismetMathLibrary.Vector_Distance2D` (`self.K2_GetActorLocation`) (`SceneComponent.K2_GetComponentLocation` (`PhysicsHandleComponent.GetGrabbedComponent` (`self.FuseComponent`)))) 3.0)) (`.SphereRadius` (`KismetSystemLibrary.GetComponentBounds` (`PhysicsHandleComponent.GetGrabbedComponent` (`self.FuseComponent`))))) (`self.SpringArmDefaultLength`) (`|EnumEquality` (`FFuseComponent.GetCurrentFuseState` (`self.FuseComponent`)) "FSTATE_FUSING")) (`local.DeltaTime`) 3.0) (`self.CameraBoom`)))
        (:`Is Not Valid`
          ;[0 0.154 0.046] If there is not a valid grabbed component, interp back to the default length
          (set `SpringArmComponent.TargetArmLength` (`KismetMathLibrary.FInterpTo` (`SpringArmComponent.TargetArmLength` (`self.CameraBoom`)) (`self.SpringArmDefaultLength`) (`local.DeltaTime`) 3.0) (`self.CameraBoom`)))))
    (:`then_1`
      ;[0 0.154 0.046] Interp the relative pitch
      (`SceneComponent.K2_SetRelativeRotation` (`self.CameraBoom`) (`KismetMathLibrary.RInterpTo` (`SceneComponent.RelativeRotation` (`self.CameraBoom`)) (`KismetMathLibrary.MakeRotator` 0.0 (`self.FusingCameraPitchTarget`)) (`local.DeltaTime`) 3.0) false false))))

(fn `DeactivateComponentArray`
  (params (Array :type "Array of PrimitiveComponent Object Reference"))
  (for _array_element Array
    (`/Engine/EditorBlueprintResources/StandardMacros.IsValid` _array_element
      (:`Is Valid`
        (`ActorComponent.Deactivate` _array_element))))
  (return))

(fn `DrawDebugInfo`
  (params (DeltaTime :type "Float (double-precision)"))
  (bind (_returnvalue_roll _returnvalue_pitch _returnvalue_yaw) (`KismetMathLibrary.BreakRotator` (`self.GetControlRotation`)))
  (`|ExecutionSequence`
    (:`then_0`
      (`self.PrintDebugFuseString` "Fuse debug active" (struct :`R` 1.0 :`A` 1.0) "Active"))
    (:`then_1`
      (`self.PrintDebugFuseString` (`KismetStringLibrary.Concat_StrStr` "Current fuse mode:  " (`|GetEnumeratorNameAsString` (`FFuseComponent.GetCurrentFuseState` (`self.FuseComponent`)))) (struct :`R` 0.004204 :`G` 0.239676 :`B` 1.0 :`A` 1.0) "State"))
    (:`then_2`
      (`self.PrintDebugFuseString` (`KismetTextLibrary.Conv_TextToString` (`|FormatText` " \nFuser relevant rotations: \nYaw: {InYaw} \nPitch dotted: {InPitch}" _returnvalue_yaw (/ (+ (`KismetMathLibrary.Dot_VectorVector` (* (`self.GetActorUpVector`) -1.0) (`KismetMathLibrary.GetForwardVector` (`self.GetControlRotation`))) 1.0) 2.0))) (struct :`R` 0.004204 :`G` 0.239676 :`B` 1.0 :`A` 1.0) "Rotations"))))

(fn `GetValueInterpTargetDeltaSeconds`
  (returns (ReturnValue :type "Float (single-precision)"))
  (return (/ 1.0 (`KismetMathLibrary.Conv_IntToDouble` (`self.InterpValueUpdateSteps`)))))

(fn `PrintDebugFuseString`
  (params (InString :type String) (TextColor :type "LinearColor Structure") (FuseDebugKey :type String))
  (`KismetSystemLibrary.PrintString` InString true false TextColor 0.5 (`KismetStringLibrary.Conv_StringToName` (`KismetStringLibrary.Concat_StrStr` "FuseDebug" FuseDebugKey))))

(fn `SetDefaultValues`
  (`|ExecutionSequence`
    (:`then_0`
      (set `self.SpringArmDefaultLength` (`SpringArmComponent.TargetArmLength` (`self.CameraBoom`))))))

(fn `UpdateFuseVisuals`
  (params (FuseState :type "EFuserState Enum" :default "FSTATE_NONE") (PreviousState :type "EFuserState Enum" :default "FSTATE_NONE"))
  (bind (_returnvalue_roll _returnvalue_pitch _returnvalue_yaw) (`KismetMathLibrary.BreakRotator` (`self.GetControlRotation`)))
  (bind (_returnvalue_roll_2 _returnvalue_pitch_2) (`KismetMathLibrary.BreakRotator` (`SceneComponent.K2_GetComponentRotation` (`self.CameraBoom`))))
  (switch `EFuserState` FuseState
    (:`FSTATE_NONE`
      (set `self.bUseControllerRotationYaw` false :!label _label)
      (`self.DeactivateComponentArray` (`self.SearchingCues`))
      (set `self.SocketOffsetTarget` (`self.SocketOffsetDefault`))
      (`Controller.SetControlRotation` (`self.GetController`) (`KismetMathLibrary.MakeRotator` _returnvalue_roll _returnvalue_pitch_2 _returnvalue_yaw))
      (set `SpringArmComponent.bInheritPitch` true (`self.CameraBoom`)))
    (:`FSTATE_SEARCHING`
      (set `self.bUseControllerRotationYaw` true)
      (bind _returnvalue (`NiagaraFunctionLibrary.SpawnSystemAttached` "/Game/Fuse/Effect/NS_FuseDecals.NS_FuseDecals" (`self.CapsuleComponent`) "None" (- (`self.K2_GetActorLocation`) (`KismetMathLibrary.MakeVector` 0.0 0.0 (`CapsuleComponent.GetScaledCapsuleHalfHeight` (`self.CapsuleComponent`)))) (`self.K2_GetActorRotation`) "KeepWorldPosition"))
      (`KismetArrayLibrary.Array_Add` (`self.SearchingCues`) _returnvalue)
      (set `self.SocketOffsetTarget` (`self.SocketOffsetFusing`)))
    (:`FSTATE_FUSING`
      (set `SpringArmComponent.bInheritPitch` false (`self.CameraBoom`))
      (`SceneComponent.K2_SetRelativeRotation` (`self.CameraBoom`) (`self.GetControlRotation`) false false))
    (:`FSTATE_ACTIVEFUSING`
      (goto _label))))

(fn `UpdateInterpValues`
  (`|ExecutionSequence`
    (:`then_0`
      (set `SpringArmComponent.SocketOffset` (`KismetMathLibrary.VInterpTo` (`SpringArmComponent.SocketOffset` (`self.CameraBoom`)) (`self.SocketOffsetTarget`) (`self.GetValueInterpTargetDeltaSeconds`) (`self.SocketInterpSpeed`)) (`self.CameraBoom`)))
    (:`then_1`
      (bind _returnvalue (`KismetMaterialLibrary.GetScalarParameterValue` "/Game/Fuse/MaterialLibrary/MPC_Fuse.MPC_Fuse" "IsFusing"))
      (`KismetMaterialLibrary.SetScalarParameterValue` "/Game/Fuse/MaterialLibrary/MPC_Fuse.MPC_Fuse" "IsFusing" (`KismetMathLibrary.FInterpTo` _returnvalue (`KismetMathLibrary.Conv_BoolToDouble` (`FFuseComponent.IsFusing` (`self.FuseComponent`))) (`self.GetValueInterpTargetDeltaSeconds`) (`self.IsFusingValueInterpSpeed`))))))

(fn `UserConstructionScript`)
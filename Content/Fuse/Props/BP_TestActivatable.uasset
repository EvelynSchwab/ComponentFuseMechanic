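; Test prop actor that pushes its skeletal mesh's physics bodies while switched on.
; Activate toggles the ShouldMove flag and prints the skeletal mesh asset's name.
; While the flag is set, Tick applies a delta-scaled impulse to all bodies below the root bone, excluding root itself.
; The forward vector is multiplied component-wise by an X-only strength vector, so the impulse acts only along world X.
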(event `Activate`
  (set `self.bShouldMove` (not (`self.bShouldMove`)))
  (`KismetSystemLibrary.PrintString` (`KismetSystemLibrary.GetDisplayName` (`SkeletalMeshComponent.GetSkeletalMeshAsset` (`self.SkeletalMesh`)))))

(event `self.ReceiveTick`
  (params (DeltaSeconds :type "Float (single-precision)"))
  (if (`self.bShouldMove`)
    (`SkeletalMeshComponent.AddImpulseToAllBodiesBelow` (`self.SkeletalMesh`) (* DeltaSeconds (* (`self.GetActorForwardVector`) (`KismetMathLibrary.MakeVector` (`self.ImpulseStrength`)))) "root" false false)))

(fn `UserConstructionScript`)